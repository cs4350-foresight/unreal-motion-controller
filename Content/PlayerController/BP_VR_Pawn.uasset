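; VR player pawn that holds health, the camera and the components for spellcasting and arc teleporting.
; On BeginPlay it initialises the motion controller component added in its construction script, then passes it to SpellController and to BPMC along with the teleport arc parts.
; Helper functions clear the arc and add spline mesh segments, choosing between two templates by location validity.
; DamagePlayer subtracts health and prints it, with no death check.
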(event `DamagePlayer`
  (params (DamagePoints :type "Float (double-precision)"))
  ;[1 1 1] Damage Player
  (bind _output_get (set `self.Health` (- (`self.Health`) DamagePoints)))
  (`KismetSystemLibrary.PrintString` (`KismetStringLibrary.Conv_DoubleToString` _output_get)))

(event `self.ReceiveBeginPlay`
  (`|ExecutionSequence`
    (:`then_0`
      ;[1 1 1] Activate Motion Controller Actor Component
      (`/Game/PlayerController/ControllerInterfaces/BPAC_Controller.Initialise` (`self.BPAC_Controller`) (`self.VR_Controller_Interface`)))
    (:`then_1`
      (`/Game/SpellSystem/SpellController.Initialise_Event` (`self.SpellController`) (`self.BPAC_Controller`))
      (`/Game/PlayerController/BPMC.InitialiseEvent` (`self.BPMC`) self (`self.BPAC_Controller`) (`self.TeleportCylinder`) (`self.ArcSplineL`) (`self.ArcSplineR`) (`self.ArcDirectionL`) (`self.ArcDirectionR`) (`self.ArcEndpoint`) (`self.Ring`)))))

(fn `AddSplineMeshComponent`
  (returns (SplineMesh :type "SplineMeshComponent Object Reference"))
  (bind _returnvalue (`KismetMathLibrary.MakeTransform` (0.0 0.0 0.0)))
  (bind _isvalidlocation (`self.IsValidLocation`))
  (if _isvalidlocation
    (bind _returnvalue_2 (`AddComponent|NODE_AddSplineMeshComponent-3` :`bManualAttachment` true :`RelativeTransform` _returnvalue)) ; Add new cylinder mesh
    (else
      (bind _returnvalue_3 (`AddComponent|NODE_AddSplineMeshComponent-4` :`bManualAttachment` true :`RelativeTransform` _returnvalue))))
  (return (select `bool` _isvalidlocation :`false` _returnvalue_3 :`true` _returnvalue_2)))

(fn `ClearArc`
  (bind _splinemeshes (`self.SplineMeshes`))
  (`ActorComponent.K2_DestroyComponent` _splinemeshes)
  (`KismetArrayLibrary.Array_Clear` _splinemeshes)
  (`SplineComponent.ClearSplinePoints` (`self.ArcSplineL`) true)
  (`SplineComponent.ClearSplinePoints` (`self.ArcSplineR`) true))

(fn `GetCamera`
  (returns (`Camera Component` :type "CameraComponent Object Reference"))
  (return (`self.Camera`)))

(fn `UserConstructionScript`
  (bind _returnvalue (`AddComponent|NODE_AddBPAC_Controller-12`))
  (set `self.BPAC_Controller` _returnvalue))